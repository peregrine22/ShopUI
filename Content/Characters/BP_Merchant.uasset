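; BP_Merchant is an interactable merchant character that opens the shop UI.
; On begin play it caches the player's BP_HUD.
; Starting interaction shows the mouse cursor, switches to UI-only input and pushes W_ShopUI onto the HUD's GameMenu layer stack.
; Ending interaction only clears the IsInteracted flag, leaving cursor and input mode untouched.
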(event `self.ReceiveBeginPlay`
  (`parent.ReceiveBeginPlay`)
  (bind _asbp_hud (cast `/Game/Blueprints/BP_HUD` (`PlayerController.GetHUD` (`GameplayStatics.GetPlayerController` 0))))
  (set `self.HUD` _asbp_hud))

(event `/Game/Blueprints/Interface/BPI_Interactable.OnInteractionStart`
  (bind _returnvalue (`GameplayStatics.GetPlayerController` 0))
  (set `self.bIsInteracted` true)
  (set `PlayerController.bShowMouseCursor` true _returnvalue)
  (`WidgetBlueprintLibrary.SetInputMode_UIOnlyEx` _returnvalue null)
  (`/Game/UI/W_Base.PushWidgetToLayerStack` (`/Game/Blueprints/BP_HUD.UIBase` (`self.HUD`)) (struct :`TagName` "UI.Layers.GameMenu") "/Game/UI/Shop/W_ShopUI.W_ShopUI_C"))

(event `/Game/Blueprints/Interface/BPI_Interactable.OnInteractionEnd`
  (set `self.bIsInteracted` false))

(fn `UserConstructionScript`)