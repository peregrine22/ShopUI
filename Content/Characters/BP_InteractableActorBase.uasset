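; BP_InteractableActorBase is a base actor for interactables that carries an interaction icon and instruction text on two widget components.
; On BeginPlay it caches the Widget component's W_Interactable and the Dialogue component's W_InteractionInstruction, passing them its icon and text variables.
; A failed first cast also skips the instruction setup.
; The ShowIcon event shows the icon, then hides it after a short delay.
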(event `self.ReceiveBeginPlay`
  (bind _asw_interactable (cast `/Game/UI/Misc/W_Interactable` (`WidgetComponent.GetUserWidgetObject` (`self.Widget`))))
  (bind _output_get (set `self.InteractableWidget` _asw_interactable))
  (`/Game/UI/Misc/W_Interactable.SetInteractionIcon` _output_get (`self.InteractionIcon`))
  (bind _asw_interaction_instruction (cast `/Game/UI/Misc/W_InteractionInstruction` (`WidgetComponent.GetUserWidgetObject` (`self.Dialogue`))))
  (bind _output_get_2 (set `self.InteractionInstructions` _asw_interaction_instruction))
  (`/Game/UI/Misc/W_InteractionInstruction.SetInteractionText` _output_get_2 (`self.InteractionText`)))

(event `/Game/Blueprints/Interface/BPI_Interactable.ShowIcon`
  (`/Game/UI/Misc/W_Interactable.ShowIcon` (`self.InteractableWidget`))
  (`KismetSystemLibrary.Delay` 3.0)
  (`/Game/UI/Misc/W_Interactable.HideIcon` (`self.InteractableWidget`)))

(fn `UserConstructionScript`)